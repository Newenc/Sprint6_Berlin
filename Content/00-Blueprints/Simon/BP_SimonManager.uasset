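; Manager for a Simon-style memory puzzle in which the player hits mushrooms to repeat a sequence of notes.
; A state variable gates input, so hits count only after delayed recursive playback of the random sequence finishes.
; Each win generates a wholly new, longer sequence, while a mistake replays the current one.
; Winning the maximum-length round marks success and calls OnSimonSolved.
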(event Custom|StartPuzzle
  (bind _output_get (Variables|Default|SetCurrentRoundLength 3))
  (CallFunction|RegenerateSequence _output_get)
  (CallFunction|StartRound))

(event Custom|OnMushroomHit
  (params (HitIndex :type Integer))
  (switch Utilities|FlowControl|Switch|SwitchonE_SimonState (Variables|Default|GetState)
    (:NewEnumerator2
      (if (== HitIndex (Utilities|Array|Get(acopy) (Variables|Default|GetSequence) (Variables|Default|GetPlayerInputIndex)))
        (Variables|Default|SetPlayerInputIndex (+ (Variables|Default|GetPlayerInputIndex) 1))
        (if (>= (Variables|Default|GetPlayerInputIndex) (Utilities|Array|Length (Variables|Default|GetSequence)))
          (CallFunction|OnRoundWon))
        (else
          (CallFunction|OnWrongAnswer))))))

(event Custom|RegenerateSequence
  (params (Length :type Integer))
  (Utilities|Array|Clear (Variables|Default|GetSequence))
  (for _index (range 0 (- Length 1))
    (Utilities|Array|Add (Variables|Default|GetSequence) (Math|Random|RandomIntegerinRange 0 (- (Utilities|Array|Length (Variables|Default|GetMushrooms)) 1))))
  (Variables|Default|SetPlayerInputIndex 0))

(event Custom|PlaySequenceStep
  (params (Index :type Integer))
  (bind _sequence (Variables|Default|GetSequence))
  (bind _mushrooms (Variables|Default|GetMushrooms))
  (bind _output (Utilities|Array|Get(acopy) _sequence Index))
  (bind _output_2 (Utilities|Array|Get(acopy) _mushrooms _output))
  (if (>= Index (Utilities|Array|Length (Variables|Default|GetSequence)))
    (Variables|Default|SetState "NewEnumerator2")
    (else
      (Utilities|IsValid _output_2
        (:Is%20Valid
          (Default|PlayNote _output_2)
          (Utilities|FlowControl|Delay 0.8)
          (CallFunction|PlaySequenceStep (+ Index 1)))))))

(event Custom|StartRound
  (for _array_element (Variables|Default|GetMushrooms)
    (Default|ResetVisualState _array_element))
  (Variables|Default|SetState "NewEnumerator1")
  (CallFunction|PlaySequenceStep))

(event Custom|OnRoundWon
  (if (>= (Variables|Default|GetCurrentRoundLength) (Variables|Default|GetMaxRoundLength))
    (CallFunction|OnPuzzleSolved)
    (else
      (Variables|Default|SetState "NewEnumerator0")
      (Variables|Default|SetCurrentRoundLength (+ (Variables|Default|GetCurrentRoundLength) 1))
      (Utilities|FlowControl|Delay 2.0)
      (CallFunction|RegenerateSequence (Variables|Default|GetCurrentRoundLength))
      (CallFunction|StartRound))))

(event Custom|OnWrongAnswer
  (Variables|Default|SetState "NewEnumerator0")
  (Variables|Default|SetPlayerInputIndex 0)
  (Utilities|FlowControl|Delay 2.0)
  (CallFunction|StartRound))

(event Custom|OnPuzzleSolved
  (Variables|Default|SetState "NewEnumerator4")
  (Default|CallOnSimonSolved))

(fn ConstructionScript)