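; BP_SimonMushroom is one mushroom in a Simon-style memory game, lit by a light component and hit by the player.
; While the manager is in the Listening state, looking at it turns the light on, and hitting it plays its note and reports its index to the manager.
; PlayNote is a timeline-driven light flash that restores the highlight afterwards if still looked at.
; ResetVisualState clears the look flag and light.
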(event Custom|OnHitFromPlayer
  (switch Utilities|FlowControl|Switch|SwitchonE_SimonState (Variables|/Game/00-Blueprints/Simon/BP_SimonManager.BP_SimonManager_C|GetState (Variables|Default|Get%20ManagerRef))
    (:NewEnumerator2
      (CallFunction|PlayNote)
      (Default|OnMushroomHit (Variables|Default|Get%20ManagerRef) (Variables|Default|GetMushroomIndex)))))

(event Custom|PlayNote
  (bind _brightness (Timeline|NoteFlashTimeline PlayFromStart)
    (:Update
      (Rendering|Components|Light|SetIntensity (Variables|Default|GetLightComponent0) (* _brightness 2e+03)))
    (:Finished
      (if (Variables|Default|Get%20IsBeingLookedAt)
        (Rendering|Components|Light|SetIntensity (Variables|Default|GetLightComponent0) 2e+03)))))

(event Custom|ResetVisualState
  (Variables|Default|Set%20IsBeingLookedAt false)
  (Rendering|Components|Light|SetIntensity (Variables|Default|GetLightComponent0) 0.0))

(event EventStartLookatInteractables
  (switch Utilities|FlowControl|Switch|SwitchonE_SimonState (Variables|/Game/00-Blueprints/Simon/BP_SimonManager.BP_SimonManager_C|GetState (Variables|Default|Get%20ManagerRef))
    (:NewEnumerator2
      (if (not (Variables|Default|Get%20IsBeingLookedAt))
        (Rendering|Components|Light|SetIntensity (Variables|Default|GetLightComponent0) 2e+03)
        (Variables|Default|Set%20IsBeingLookedAt true)))))

(event EventStopLookatInteractables
  (if (Variables|Default|Get%20IsBeingLookedAt)
    (Variables|Default|Set%20IsBeingLookedAt false)
    (Rendering|Components|Light|SetIntensity (Variables|Default|GetLightComponent0) 0.0)))

(fn ConstructionScript)